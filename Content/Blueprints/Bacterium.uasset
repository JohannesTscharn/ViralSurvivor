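; Bacterium is an actor that acts as a buff pickup for the virus, consumed on proximity.
; Each Tick it measures its distance to the VirusClass reference and, within a small fixed radius, sets that virus's IsBuffed flag and destroys itself.
; Detection relies on this polling, as the overlap event is empty.
; Leftover, disconnected nodes hint at interpolated movement toward a Target, but they never run.
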(event EventBeginPlay)

(event Collision|EventActorBeginOverlap
  (params (OtherActor :type Actor%20Object%20Reference)))

(event EventTick
  (params (DeltaSeconds :type Float%20%28single-precision%29))
  (if (< (Math|Vector|Distance(Vector) (Transformation|GetActorLocation) (Transformation|GetActorLocation (Variables|Default|GetVirusClass))) 5e+01)
    (Variables|/Game/VirtualReality/VirtualRealityBP/Blueprints/BP_PickupCube.BP_PickupCube_C|SetIsBuffed (Variables|Default|GetVirusClass) true)
    (Actor|DestroyActor)))

(fn ConstructionScript)