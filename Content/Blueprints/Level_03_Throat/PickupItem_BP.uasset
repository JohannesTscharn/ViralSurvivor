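; VR pickup actor in the Throat level that wanders randomly around its spawn point until grabbed.
; Tick lerps it toward a target with sweep, while a random Delay gates picking a new target within MaxRndMovementRange and snapping rotation along that line.
; BP_MotionController calls Pickup to attach it and pause wandering.
; Drop detaches it with physics still off, so it resumes drifting around the original start position.
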(event EventBeginPlay
  ;[0.2944 0.6341 1] Random Movement
  ;;[1 1 1] Set Variable Vectors / Positions
  (bind _output_get (Variables|Default|SetStartPos (Transformation|GetActorLocation)))
  (Variables|Default|SetTargetPos _output_get))

(event Collision|EventActorBeginOverlap
  (params (OtherActor :type Actor%20Object%20Reference)))

(event EventTick
  (params (DeltaSeconds :type Float%20%28single-precision%29))
  (bind _startpos (Variables|Default|GetStartPos))
  (bind _maxrndmovementrange (Variables|Default|GetMaxRndMovementRange))
  (bind _returnvalue (* _maxrndmovementrange -1.0))
  ;[0.2944 0.6341 1] Random Movement
  ;;[1 1 1] Only move randomly when not Picked Up
  (if (not (Variables|Default|GetPickedUp))
    ;;[1 1 1] Set Variable Vectors / Positions
    (bind _output_get (Variables|Default|SetCurrentPos (Transformation|GetActorLocation)))
    ;;[1 1 1] Lerp to Target Location
    (Transformation|SetActorLocation (Math|Vector|Lerp(Vector) _output_get (Variables|Default|GetTargetPos) 0.05) true false)
    ;;[1 1 1] Random Length Delay
    (Utilities|FlowControl|Delay (Math|Random|RandomFloatinRange 0.5 4.0))
    ;;[1 1 1] Move to Random Location / Set Random Location
    (bind _output_get_2 (Variables|Default|SetRandomPos (Math|Vector|MakeVector (+ (Math|Random|RandomFloatinRange _returnvalue _maxrndmovementrange) (.x _startpos)) (+ (Math|Random|RandomFloatinRange _returnvalue _maxrndmovementrange) (.y _startpos)) (+ (Math|Random|RandomFloatinRange _returnvalue _maxrndmovementrange) (.z _startpos)))))
    (Variables|Default|SetTargetPos _output_get_2)
    ;;;[1 1 1] Rotate towards Target
    (Transformation|SetActorRotation (Math|Conversions|RotationFromXVector (- (Variables|Default|GetCurrentPos) (Variables|Default|GetRandomPos))))))

(event EventPickup
  (params (AttachTo :type Scene%20Component%20Object%20Reference))
  ;[1 1 1] Pickup / Drop
  (Variables|Default|SetPickedUp true)
  (Physics|SetSimulatePhysics (Variables|Debug|GetStaticMeshComponent) false)
  (Transformation|AttachComponentToComponent (VehicleSound|GetRootComponent) AttachTo "None" "KeepWorld" "KeepWorld" "KeepWorld" false))

(event EventDrop
  ;[1 1 1] Pickup / Drop
  (Variables|Default|SetPickedUp false)
  (Physics|SetSimulatePhysics (Variables|Debug|GetStaticMeshComponent) false)
  (Transformation|DetachFromActor "KeepWorld" "KeepWorld" "KeepWorld"))

(fn ConstructionScript)