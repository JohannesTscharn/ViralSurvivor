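; Climbable VR vein actor, built in the construction script as collidable spline meshes in fixed-length sections along a spline.
; Climb and LetGo track up to two motion controllers, using the newest grip as pivot and updating the pawn's climbing hand count.
; Tick offsets the climbing pawn to keep that controller at the pivot.
; Tick also switches segment materials between unlit, partly lit and fully lit states.
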(event EventBeginPlay)

(event Collision|EventActorBeginOverlap
  (params (OtherActor :type Actor%20Object%20Reference)))

(event EventTick
  (params (DeltaSeconds :type Float%20%28single-precision%29))
  (bind _firstmotioncontroller (Variables|Default|GetFirstMotionController))
  (bind _secondmotioncontroller (Variables|Default|GetSecondMotionController))
  (bind _secondmotioncontroller_2 (Variables|Default|GetSecondMotionController))
  (bind _mcpawn (Variables|Default|GetMCPawn))
  (bind _returnvalue (Utilities|IsValid _secondmotioncontroller_2))
  (bind _returnvalue_2 (select _returnvalue _secondmotioncontroller _firstmotioncontroller))
  ;[0.4121 0.7086 1] Set Material based on LightStates
  (for _array_element (Variables|Default|GetSplineMeshes)
    ;;[1 1 1] Check Light State
    (if (Variables|Default|GetPartLit)
      (if (Variables|Default|GetFullyLit)
        (Rendering|Material|SetMaterial _array_element 0 "/Game/Assets/Materials/Stage_01/VeinstLit_Inst.VeinstLit_Inst")
        (else
          (Rendering|Material|SetMaterial _array_element 0 "/Game/Assets/Materials/Stage_01/VeinsPartLit_Inst.VeinsPartLit_Inst")))
      (else
        (Rendering|Material|SetMaterial _array_element 0 "/Game/Assets/Materials/Stage_01/Veins.Veins")))
    ;[0.4121 0.7086 1] Climbing Transform
    ;;[1 1 1] Check if Pawn + MC is Valid / not climbing
    (if (Utilities|IsValid _mcpawn)
      (if (and (Variables|/Game/VirtualReality/VirtualRealityBP/Blueprints/MotionControllerPawn.MotionControllerPawn_C|GetPawnIsClimbing _mcpawn) (Utilities|IsValid (Variables|Default|GetFirstMotionController)))
        ;;[1 1 1] Apply Transform to MC Pawn
        (Transformation|AddActorWorldOffset (Variables|Default|GetMCPawn) (- (Variables|Default|GetPivot) (Transformation|GetWorldLocation _returnvalue_2)))
        ;;[1 1 1] Apply Transform to Motion Controller
        (Transformation|SetWorldLocation _returnvalue_2 (Variables|Default|GetPivot) false false)))))

(event EventClimb
  (params (Motion%20Controller :type Scene%20Component%20Object%20Reference))
  ;[0.4121 0.7086 1] Climb
  ;;[1 1 1] Check if Grabbed by one or two Controllers
  (if (Utilities|IsValid (Variables|Default|GetFirstMotionController))
    (Variables|Default|SetSecondMotionController Motion%20Controller)
    (else
      (Variables|Default|SetFirstMotionController Motion%20Controller)))
  ;;[1 1 1] Determine Controller to use as Pivot (if two, second is Pivot)
  (Variables|Default|SetPivot (Transformation|GetWorldLocation (select (Utilities|IsValid (Variables|Default|GetSecondMotionController)) (Variables|Default|GetSecondMotionController) (Variables|Default|GetFirstMotionController))))
  ;;[1 1 1] Get MC Pawn / Increment Climbing Hands
  (bind _asmotion_controller_pawn (Utilities|Casting|CastToMotionControllerPawn (Game|Player|GetPlayerPawn 0)))
  (bind _output_get (Variables|Default|SetMCPawn _asmotion_controller_pawn))
  (Math|Integer|IncrementInt (Variables|/Game/VirtualReality/VirtualRealityBP/Blueprints/MotionControllerPawn.MotionControllerPawn_C|GetClimbingHands _output_get)))

(event EventLetGo
  (params (Motion%20Controller :type Scene%20Component%20Object%20Reference))
  ;[0.4121 0.7086 1] Let Go
  ;;[1 1 1] Determine which Hand to Let go
  (if (Utilities|IsValid (Variables|Default|GetSecondMotionController))
    (if (== (Variables|Default|GetSecondMotionController) Motion%20Controller)
      ;;[1 1 1] Two Hands: Second MC is Current -> Reset Second MC / Set Pivot to First
      (Variables|Default|SetSecondMotionController 0)
      (Variables|Default|SetPivot (Transformation|GetWorldLocation (Variables|Default|GetFirstMotionController)))
      (else
        ;;[1 1 1] Two Hands: First MC is Current -> Set Second to First / Set Pivot to new First
        (Variables|Default|SetFirstMotionController (Variables|Default|GetSecondMotionController))
        (Variables|Default|SetSecondMotionController 0)
        (Variables|Default|SetPivot (Transformation|GetWorldLocation (Variables|Default|GetFirstMotionController)))))
    ;;[1 1 1] Get MC Pawn / Decrement Climbing Hands
    (Math|Integer|DecrementInt (Variables|/Game/VirtualReality/VirtualRealityBP/Blueprints/MotionControllerPawn.MotionControllerPawn_C|GetClimbingHands (Variables|Default|GetMCPawn)) :!label _label)
    (elif (== Motion%20Controller (Variables|Default|GetFirstMotionController))
      ;;[1 1 1] One Hand: Reset All
      (Variables|Default|SetFirstMotionController 0)
      (Variables|Default|SetSecondMotionController 0)
      (Variables|Default|SetPivot "0, 0, 0")
      (goto _label))))

(fn ConstructionScript
  (bind _spline (Variables|Default|GetSpline))
  (bind _spline_2 (Variables|Default|GetSpline))
  ;[0.4688 0.7795 1] Loop over all Spline points
  (for _index (range 0 (Math|Float|Truncate (/ (Spline|GetSplineLength (Variables|Default|GetSpline)) (Variables|Default|GetSectionLength))))
    ;;[1 1 1] Add and configure SplineMesh Component
    (bind _returnvalue (AddComponent|AddSplineMeshComponent false))
    (Utilities|Array|Add (Variables|Default|GetSplineMeshes) _returnvalue)
    (SplineMesh|SetForwardAxis _returnvalue "Z" true)
    (Collision|SetCollisionEnabled _returnvalue "QueryAndPhysics")
    (SplineMesh|SetStartandEnd _returnvalue (Spline|GetLocationatDistanceAlongSpline _spline_2 (* _index (Variables|Default|GetSectionLength)) "Local") (Math|Vector|ClampVectorSize (Spline|GetTangentatDistanceAlongSpline _spline_2 (* _index (Variables|Default|GetSectionLength)) "Local") 0.0 (Variables|Default|GetSectionLength)) (Spline|GetLocationatDistanceAlongSpline _spline (* (+ _index 1) (Variables|Default|GetSectionLength)) "Local") (Math|Vector|ClampVectorSize (Spline|GetTangentatDistanceAlongSpline _spline (* (+ _index 1) (Variables|Default|GetSectionLength)) "Local") 0.0 (Variables|Default|GetSectionLength)) true :!class /Script/Engine.SplineMeshComponent)))