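; FogController is a Stage 01 Blueprint that pushes the height fog back as junctions are activated.
; DecreaseFogRange raises the target fog start distance by an increment and doubles each registered vein's build-up distance; final junctions instead set a fixed target and increment a counter.
; Tick steps the current distance up by one per frame while it differs from the target.
; AppendToVeinList registers veins without duplicates.
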(event EventBeginPlay)

(event EventTick
  (params (DeltaSeconds :type Float%20%28single-precision%29))
  (if (!= (Variables|Default|GetStartDistance_Current) (Variables|Default|GetStartDistance_Target))
    (bind _result (Math|Float|IncrementFloat (Variables|Default|GetStartDistance_Current))
      (:%20%20
        (Class|ExponentialHeightFogComponent|SetStartDistance (Variables|/Script/Engine.ExponentialHeightFog|GetComponent (Variables|Default|GetExponHeight_Fog)) _result)))))

(fn ConstructionScript)

(fn DecreaseFogRange
  (params (FinalJunction :type Boolean))
  (if FinalJunction
    (Math|Integer|IncrementInt (Variables|Default|GetFinalJunctionsActivated)
      (:%20%20
        (Variables|Default|SetStartDistance_Target 5e+03)))
    (else
      ;[1 1 1] Increment FogStartDistance
      (Variables|Default|SetStartDistance_Target (+ (Variables|Default|GetStartDistance_Current) (Variables|Default|GetStartDistance_Increments)))
      ;[1 1 1] Increase Visibility Range of already Activated Veins
      (for _array_element (Variables|Default|GetActiveVeins)
        (Variables|/Game/Blueprints/Stage_01/Vein_BP.Vein_BP_C|SetVein_BuildUpDistance _array_element (* (Variables|/Game/Blueprints/Stage_01/Vein_BP.Vein_BP_C|GetVein_BuildUpDistance _array_element) 2.0))))))

(fn AppendtoVeinList
  (params (Vein :type Array%20of%20Vein%20BP%20Object%20References))
  (for _array_element Vein
    (Utilities|Array|AddUnique (Variables|Default|GetActiveVeins) _array_element)))