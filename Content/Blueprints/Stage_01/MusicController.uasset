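; Stage 01 music controller that layers in audio tracks according to an active-track count, apparently raised as bacteria are collected.
; BeginPlay drops every track in the Music array to near-silence.
; While MusicTracksActive is positive, Tick re-issues a logarithmic fade-up on every track with an index below that count minus one.
; Nothing here changes the count or fades tracks back down.
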(event EventBeginPlay
  ;[0.4546 0.7407 1] Set Music Volume to 0
  (for _array_element (Variables|Default|GetMusic)
    (Audio|Components|Audio|AdjustVolume (Variables|/Script/Engine.AmbientSound|GetAudioComponent _array_element) 0.0 0.001 "Linear" :!class /Script/Engine.AudioComponent)))

(event Collision|EventActorBeginOverlap
  (params (OtherActor :type Actor%20Object%20Reference)))

(event EventTick
  (params (DeltaSeconds :type Float%20%28single-precision%29))
  ;[0.4546 0.7407 1] Trigger BactCollected Music Change
  (if (> (Variables|Default|GetMusicTracksActive) 0)
    ;;[1 1 1] Loop Over MusicArray
    (for (_array_element _array_index) (Variables|Default|GetMusic)
      (if (< _array_index (- (Variables|Default|GetMusicTracksActive) 1))
        (Audio|Components|Audio|AdjustVolume (Variables|/Script/Engine.AmbientSound|GetAudioComponent _array_element) 3.0 0.75 "Logarithmic" :!class /Script/Engine.AudioComponent)))))

(fn ConstructionScript)