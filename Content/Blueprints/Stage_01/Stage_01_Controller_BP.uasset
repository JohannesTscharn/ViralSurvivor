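; Stage 01 level controller that starts music and reacts to bacteria collection in a motion-controller game.
; Tick starts the music once the tutorial completes, having stopped it on BeginPlay.
; Tick also steps toward the collected-bacteria total, flagging MusicController, widening global visibility range and thinning height fog down to a threshold on each step.
; Controller references are cached on BeginPlay; their validation is disconnected, and IncrementBactCollected is an empty stub.
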(event EventBeginPlay
  (bind _motioncontrollerpawn (Variables|Default|GetMotionControllerPawn))
  (Variables|Default|SetBP_MotionController_L (Variables|/Game/VirtualReality/VirtualRealityBP/Blueprints/MotionControllerPawn.MotionControllerPawn_C|GetLeftController _motioncontrollerpawn))
  (Variables|Default|SetBP_MotionController_R (Variables|/Game/VirtualReality/VirtualRealityBP/Blueprints/MotionControllerPawn.MotionControllerPawn_C|GetRightController _motioncontrollerpawn))
  (Audio|Components|Audio|Stop (Variables|/Script/Engine.AmbientSound|GetAudioComponent (Variables|Default|GetMusic))))

(event Collision|EventActorBeginOverlap
  (params (OtherActor :type Actor%20Object%20Reference)))

(event EventTick
  (params (DeltaSeconds :type Float%20%28single-precision%29))
  (bind _exponheightfog (Variables|Default|GetExponHeightFog))
  (bind _previousbactcollected (Variables|Default|GetPreviousBactCollected))
  (bind _component (Variables|/Script/Engine.ExponentialHeightFog|GetComponent _exponheightfog))
  (bind _fogdensity (Variables|/Script/Engine.ExponentialHeightFogComponent|GetFogDensity _component))
  ;[0.4948 0.8192 1] Music
  (if (Variables|/Game/Blueprints/Stage_01/Stage_01_LocomotionTutorial.Stage_01_LocomotionTutorial_C|GetTutorialCompleted (Variables|Default|GetTutorialController))
    (if (Variables|Default|GetMusicPlaying)
      _
      (else
        ;;[1 1 1] Start Playing Music
        (Audio|Components|Audio|Play (Variables|/Script/Engine.AmbientSound|GetAudioComponent (Variables|Default|GetMusic)) 0.0)
        (Variables|Default|SetMusicPlaying true))))
  ;[0.4948 0.8192 1] Check if MotionControllers are Assigned
  (if (Variables|Default|GetMotionControllersAssigned)
    _
    (else
      _))
  ;[0.4948 0.8192 1] Check / Iterate total BacteriaCounter
  (if (> (Variables|Default|GetTotalBactCollected) _previousbactcollected)
    (Math|Integer|IncrementInt _previousbactcollected
      (:%20%20
        ;;[1 1 1] Propagate Change to MusicController
        (Variables|/Game/Blueprints/Stage_01/MusicController.MusicController_C|SetBactCollected (Variables|Default|GetMusicController) true)
        ;;[1 1 1] Handle Dynamic Visibility Range
        (Variables|Default|SetGlobalVisibilityRange (* (Variables|Default|GetGlobalVisibilityRange) 1.25))
        (if (> _fogdensity 0.05)
          (Class|ExponentialHeightFogComponent|SetFogDensity _component (* _fogdensity 0.5)))))))

(fn ConstructionScript)

(fn IncrementBactCollected)