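; A bacterium wall light that brightens each time a picked-up bacterium item overlaps it and is consumed.
; Each one destroys the item, resets the Niagara effect and raises a counter driving spotlight and optional extra light intensity.
; The mesh pulses via timeline, scaled by that counter and, until first fed, by VR pawn proximity.
; Tutorial mode replaces this pulse with a prompt and pulsing sphere while the tutorial bacterium is held.
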(event EventBeginPlay
  ;[0.4455 0.7411 1] Setup Initial Values
  (Rendering|Components|Light|SetIntensity (Variables|Default|GetSpotLight) 0.0)
  (Rendering|Material|SetMaterial (Variables|Default|GetVisibleMesh) 0 "/Game/Materials/CollectibleBacterium_M_2.CollectibleBacterium_M_2")
  (Class|NiagaraComponent|SetPaused (Variables|Default|GetNiagara) true)
  ;[0.4455 0.7411 1] Get Player (MC) Pawn
  (bind _asmotion_controller_pawn (Utilities|Casting|CastToMotionControllerPawn (Game|Player|GetPlayerPawn 0)))
  (Variables|Default|SetMCPawn _asmotion_controller_pawn)
  ;[0.4455 0.7411 1] Additional LightSource Case
  (if (Variables|Default|GetEnableAdditionalLightsource)
    (Rendering|Components|Light|SetIntensity (Variables|/Script/Engine.Light|GetLightComponent (Variables|Default|GetAdditionalLightsource)) 0.0)))

(event Collision|EventActorBeginOverlap
  (params (OtherActor :type Actor%20Object%20Reference))
  (bind _niagara (Variables|Default|GetNiagara))
  ;[0.4455 0.7411 1] Handle Bacterium Pickup
  ;;[1 1 1] Destroy Other if PickedUp Bacterium
  (bind _aspickup_item_bp (Utilities|Casting|CastToPickupItem_BP OtherActor))
  (if true
    (if (Variables|/Game/Blueprints/Stage_01/PickupItem_BP.PickupItem_BP_C|GetPickedUp _aspickup_item_bp)
      (Actor|DestroyActor OtherActor)
      ;;[1 1 1] Play Particle Simulation
      (Class|NiagaraComponent|SetPaused _niagara true)
      (Niagara|ResetSystem _niagara)
      ;;[1 1 1] Iterate BuffCounter
      (bind _output_get (Variables|Default|SetBuffCounter (+ (Variables|Default|GetBuffCounter) 1.0)))
      ;;[1 1 1] Set SpotLight Intensity based on BuffCounter
      (Rendering|Components|Light|SetIntensity (Variables|Default|GetSpotLight) (* _output_get 1.5e+04))
      ;;[1 1 1] Additional LightSource Case
      (if (Variables|Default|GetEnableAdditionalLightsource)
        (Rendering|Components|Light|SetIntensity (Variables|/Script/Engine.Light|GetLightComponent (Variables|Default|GetAdditionalLightsource)) (* _output_get 1.5e+04))))))

(event EventTick
  (params (DeltaSeconds :type Float%20%28single-precision%29))
  (bind _visiblemesh (Variables|Default|GetVisibleMesh))
  (bind _tutorialbacterium (Variables|Default|GetTutorialBacterium))
  (if (Variables|Default|GetTutorialModeEnabled)
    (if (Utilities|IsValid _tutorialbacterium)
      (if (Variables|/Game/Blueprints/Stage_01/PickupItem_BP.PickupItem_BP_C|GetPickedUp _tutorialbacterium)
        ;[1 1 1] Enable Tutorial Elements
        (Rendering|Components|TextRender|SetText (Variables|Default|GetTutorialText) (Utilities|Text|ToText(String) "Put the Bacterium here"))
        (bind _scalepulsetrack (Timeline|TutorialPulseScale Play)
          (:Update
            (Transformation|SetRelativeScale3D (Variables|Default|GetTutorialSphere) (Math|Conversions|ToVector(Float) _scalepulsetrack))))
        (else
          ;[1 1 1] Disable Tutorial Elements
          (Rendering|Components|TextRender|SetText (Variables|Default|GetTutorialText) (Utilities|Text|ToText(String) "") :!label _label)
          (Transformation|SetRelativeScale3D (Variables|Default|GetTutorialSphere) "0, 0, 0")
          (Audio|Components|Audio|Stop (Variables|Default|GetTutorialPulseScale))))
      (else
        (goto _label)))
    (else
      ;[0.4455 0.7411 1] Update Distance to MCPawn
      (Variables|Default|SetDistToPawn (Transformation|GetDistanceTo (Variables|Default|GetMCPawn)))
      ;[0.4455 0.7411 1] Pulse Scale
      (bind _scale (Timeline|PulseScale Play)
        (:Update
          (if (> (Variables|Default|GetBuffCounter) 0.0)
            (Transformation|SetRelativeScale3D _visiblemesh (Math|Conversions|ToVector(Float) (* _scale (Math|Float|MapRangeClamped (Variables|Default|GetBuffCounter) 0.0 3.0 0.25 0.5))))
            (else
              (Transformation|SetRelativeScale3D _visiblemesh (Math|Conversions|ToVector(Float) (* (* _scale (Math|Float|MapRangeClamped (Variables|Default|GetBuffCounter) 0.0 3.0 0.25 0.5)) (Math|Float|MapRangeClamped (Variables|Default|GetDistToPawn) 1.5e+03 2.5e+02 0.01 1.0)))))))))))

(fn ConstructionScript)