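; PickupItem_BP is a bacterium pickup that BP_MotionController can grab, shifting its look to infected while held and disinfected once dropped.
; Timelines drive color, emission and movement speed values, which Tick pushes into a dynamic material instance.
; While free, it drifts by interpolating toward random points around its start position.
; Pickup attaches it to the given component; Drop detaches it and re-centers the wandering.
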(event EventBeginPlay
  (bind _returnvalue (Rendering|Material|CreateDynamicMaterialInstance (Variables|Debug|GetStaticMeshComponent) 0 "/Game/Assets/Materials/Stage_01/Bacterium_Infected.Bacterium_Infected" "None" :!class /Script/Engine.PrimitiveComponent))
  (Variables|Shader|SetDynamicMaterialInstance _returnvalue)
  (Rendering|Material|SetMaterial (Variables|Debug|GetStaticMeshComponent) 0 (Variables|Shader|GetDynamicMaterialInstance))
  (Variables|RandomMovement|SetStartPos (Transformation|GetWorldLocation (Variables|Debug|GetStaticMeshComponent))))

(event EventTick
  (params (DeltaSeconds :type Float%20%28single-precision%29))
  (bind _dynamicmaterialinstance (Variables|Shader|GetDynamicMaterialInstance))
  (Rendering|Material|SetVectorParameterValue _dynamicmaterialinstance "Color" (Math|Conversions|ToLinearColor(Color) (Variables|Shader|GetM_Color)) :!class /Script/Engine.MaterialInstanceDynamic)
  (Rendering|Material|SetScalarParameterValue _dynamicmaterialinstance "Emission" (Variables|Shader|GetM_Emission) :!class /Script/Engine.MaterialInstanceDynamic)
  (Rendering|Material|SetScalarParameterValue _dynamicmaterialinstance "EmissionSecond" (Variables|Shader|GetM_EmissionSecond) :!class /Script/Engine.MaterialInstanceDynamic)
  (Rendering|Material|SetScalarParameterValue _dynamicmaterialinstance "MovementSpeed" (Variables|Shader|GetM_MovementSpeed) :!class /Script/Engine.MaterialInstanceDynamic)
  (if (Variables|Default|GetPickedUp)
    (bind (_direction _color _emission _movementspeed) (Timeline|Infect_Material Play)
      (:Update
        (Variables|Shader|SetM_Color (Math|Conversions|ToColor(LinearColor) _color))
        (Variables|Shader|SetM_EmissionSecond _emission)
        (Variables|Shader|SetM_Emission _emission)
        (Variables|Shader|SetM_MovementSpeed _movementspeed)))
    (else
      (CallFunction|RndMovement)
      (bind (_direction_2 _color_2 _emission_2) (Timeline|Disinfect_Material Play)
        (:Update
          (Variables|Shader|SetM_Color (Math|Conversions|ToColor(LinearColor) _color_2))
          (bind _output_get (Variables|Shader|SetM_EmissionSecond _emission_2))
          (Variables|Shader|SetM_Emission (* _output_get 0.02))
          (Variables|Shader|SetM_MovementSpeed (Math|Float|MapRangeClamped _emission_2 2.0 15.0 0.05 0.02)))))))

(event EventPickup
  (params (AttachTo :type Scene%20Component%20Object%20Reference))
  ;[0.2944 0.6341 1] Pickup
  (Variables|Default|SetPickedUp true)
  (Physics|SetSimulatePhysics (Variables|Debug|GetStaticMeshComponent) false)
  (Transformation|AttachComponentToComponent (VehicleSound|GetRootComponent) AttachTo "None" "SnapToTarget" "SnapToTarget" "KeepWorld" false)
  (Components|Timeline|PlayfromStart (Variables|Default|GetInfect_Material)))

(event EventDrop
  ;[0.2944 0.6341 1] Drop
  (Physics|SetSimulatePhysics (Variables|Debug|GetStaticMeshComponent) false)
  (Transformation|DetachFromActor "KeepWorld" "KeepWorld" "KeepWorld")
  (Variables|Default|SetPickedUp false)
  (Components|Timeline|PlayfromStart (Variables|Default|GetDisinfect_Material))
  ;;[1 1 1] Reset RndMovement origin
  (Variables|RandomMovement|SetStartPos (Transformation|GetWorldLocation (Variables|Debug|GetStaticMeshComponent)))
  (Variables|RandomMovement|SetRndPos "0, 0, 0"))

(fn ConstructionScript)

(fn RndMovement
  (bind _maxrndmovement (Variables|RandomMovement|GetMaxRndMovement))
  (bind _startpos (Variables|RandomMovement|GetStartPos))
  (bind _returnvalue (* _maxrndmovement -1.0))
  (Variables|RandomMovement|SetCurrentPos (Transformation|GetWorldLocation (Variables|Debug|GetStaticMeshComponent)))
  (if (Math|Vector|Equal(Vector) (Variables|RandomMovement|GetRndPos) "0, 0, 0" 1.0)
    ;[1 1 1] New RndPos
    (Variables|RandomMovement|SetRndPos (Math|Vector|MakeVector (+ (.x _startpos) (Math|Random|RandomFloatinRange _returnvalue _maxrndmovement)) (+ (.y _startpos) (Math|Random|RandomFloatinRange _returnvalue _maxrndmovement)) (+ (.z _startpos) (Math|Random|RandomFloatinRange _returnvalue _maxrndmovement))) :!label _label)
    (else
      ;[1 1 1] Interpolate to new Position
      (Transformation|SetActorLocation (Math|Interpolation|VInterpTo (Variables|RandomMovement|GetCurrentPos) (Variables|RandomMovement|GetRndPos) (Utilities|Time|GetWorldDeltaSeconds) (Variables|RandomMovement|GetMovementSpeed)) false false)
      (if (Math|Vector|Equal(Vector) (Variables|RandomMovement|GetCurrentPos) (Variables|RandomMovement|GetRndPos) 2.0)
        (goto _label)))))