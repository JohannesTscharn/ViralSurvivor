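; Stage 01 vein extension actor: a spline-shaped vein whose material lights up when the extension is activated.
; The construction script splits the spline into fixed-length, collidable spline mesh segments with clamped tangents.
; Every Tick creates a new dynamic material per segment, zeroing its glow when inactive.
; When active, it sets full illumination and raises a shared distance divider once per segment until a threshold, then snaps to maximum.
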(event EventBeginPlay)

(event Collision|EventActorBeginOverlap
  (params (OtherActor :type Actor%20Object%20Reference)))

(event EventTick
  (params (DeltaSeconds :type Float%20%28single-precision%29))
  ;[0.4121 0.7086 1] Material
  (for _array_element (Variables|Default|GetSplineMeshes)
    (bind _returnvalue (Rendering|Material|CreateDynamicMaterialInstance "/Game/Assets/Materials/Stage_01/Veins.Veins" "None" :!class /Script/Engine.KismetMaterialLibrary))
    (Rendering|Material|SetMaterial _array_element 0 _returnvalue)
    ;;[1 1 1] Vein Active?
    (if (Variables|Default|GetExtensionActivated)
      ;;[1 1 1] BuildUp Sequence
      (if (< (Variables|Default|GetVeinDistanceDivider) 1.5e+03)
        (Variables|Default|SetVeinDistanceDivider (+ (Variables|Default|GetVeinDistanceDivider) 0.25))
        (else
          (Variables|Default|SetVeinDistanceDivider 2.5e+03)))
      ;;[1 1 1] Emission Amount based on Vein-State
      (Rendering|Material|SetScalarParameterValue _returnvalue "DistanceDivider" (Variables|Default|GetVeinDistanceDivider) :!class /Script/Engine.MaterialInstanceDynamic)
      (Rendering|Material|SetScalarParameterValue _returnvalue "TotalIllumIntensity" 125.0 :!class /Script/Engine.MaterialInstanceDynamic)
      (else
        (Rendering|Material|SetScalarParameterValue _returnvalue "TotalIllumIntensity" 0.0 :!class /Script/Engine.MaterialInstanceDynamic)
        (Rendering|Material|SetScalarParameterValue _returnvalue "DistanceDivider" 0.0 :!class /Script/Engine.MaterialInstanceDynamic)))))

(fn ConstructionScript
  (bind _spline (Variables|Default|GetSpline))
  (bind _spline_2 (Variables|Default|GetSpline))
  ;[0.4688 0.7795 1] Loop over all Spline points
  (for _index (range 0 (Math|Float|Truncate (/ (Spline|GetSplineLength (Variables|Default|GetSpline)) (Variables|Default|GetSectionLength))))
    ;;[1 1 1] Add and configure SplineMesh Component
    (bind _returnvalue (AddComponent|AddSplineMeshComponent false))
    (Utilities|Array|Add (Variables|Default|GetSplineMeshes) _returnvalue)
    (SplineMesh|SetForwardAxis _returnvalue "Y" true)
    (Collision|SetCollisionEnabled _returnvalue "QueryAndPhysics")
    (SplineMesh|SetStartandEnd _returnvalue (Spline|GetLocationatDistanceAlongSpline _spline_2 (* _index (Variables|Default|GetSectionLength)) "Local") (Math|Vector|ClampVectorSize (Spline|GetTangentatDistanceAlongSpline _spline_2 (* _index (Variables|Default|GetSectionLength)) "Local") 0.0 (Variables|Default|GetSectionLength)) (Spline|GetLocationatDistanceAlongSpline _spline (* (+ _index 1) (Variables|Default|GetSectionLength)) "Local") (Math|Vector|ClampVectorSize (Spline|GetTangentatDistanceAlongSpline _spline (* (+ _index 1) (Variables|Default|GetSectionLength)) "Local") 0.0 (Variables|Default|GetSectionLength)) true :!class /Script/Engine.SplineMeshComponent)))