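; ClimbableSurface_BP is a VR climbable surface that lets the player pull the MotionControllerPawn around by gripping with one or two motion controllers.
; Climb and LetGo track the gripping hands, update the pawn's ClimbingHands count and set a Pivot from the most recent remaining grip.
; While climbing, Tick offsets the pawn by the pivot-to-controller delta and pins that controller at the Pivot, so hand movement moves the body inversely.
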(event EventBeginPlay)

(event Collision|EventActorBeginOverlap
  (params (OtherActor :type Actor%20Object%20Reference)))

(event EventTick
  (params (DeltaSeconds :type Float%20%28single-precision%29))
  (bind _firstmotioncontroller (Variables|Default|GetFirstMotionController))
  (bind _secondmotioncontroller (Variables|Default|GetSecondMotionController))
  (bind _secondmotioncontroller_2 (Variables|Default|GetSecondMotionController))
  (bind _mcpawn (Variables|Default|GetMCPawn))
  (bind _returnvalue (Utilities|IsValid _secondmotioncontroller_2))
  (bind _returnvalue_2 (select _returnvalue _secondmotioncontroller _firstmotioncontroller))
  ;[0.4121 0.7086 1] Climbing Transform
  ;;[1 1 1] Check if Pawn + MC is Valid / not climbing
  (if (Utilities|IsValid _mcpawn)
    (if (and (Variables|/Game/VirtualReality/VirtualRealityBP/Blueprints/MotionControllerPawn.MotionControllerPawn_C|GetPawnIsClimbing _mcpawn) (Utilities|IsValid (Variables|Default|GetFirstMotionController)))
      ;;[1 1 1] Apply Transform to MC Pawn
      (Transformation|AddActorWorldOffset (Variables|Default|GetMCPawn) (- (Variables|Default|GetPivot) (Transformation|GetWorldLocation _returnvalue_2)))
      ;;[1 1 1] Apply Transform to Motion Controller
      (Transformation|SetWorldLocation _returnvalue_2 (Variables|Default|GetPivot) false false))))

(event EventClimb
  (params (Motion%20Controller :type Scene%20Component%20Object%20Reference))
  ;[0.4121 0.7086 1] Climb
  ;;[1 1 1] Check if Grabbed by one or two Controllers
  (if (Utilities|IsValid (Variables|Default|GetFirstMotionController))
    (Variables|Default|SetSecondMotionController Motion%20Controller)
    (else
      (Variables|Default|SetFirstMotionController Motion%20Controller)))
  ;;[1 1 1] Determine Controller to use as Pivot (if two, second is Pivot)
  (Variables|Default|SetPivot (Transformation|GetWorldLocation (select (Utilities|IsValid (Variables|Default|GetSecondMotionController)) (Variables|Default|GetSecondMotionController) (Variables|Default|GetFirstMotionController))))
  ;;[1 1 1] Get MC Pawn / Increment Climbing Hands
  (bind _asmotion_controller_pawn (Utilities|Casting|CastToMotionControllerPawn (Game|Player|GetPlayerPawn 0)))
  (bind _output_get (Variables|Default|SetMCPawn _asmotion_controller_pawn))
  (Math|Integer|IncrementInt (Variables|/Game/VirtualReality/VirtualRealityBP/Blueprints/MotionControllerPawn.MotionControllerPawn_C|GetClimbingHands _output_get)))

(event EventLetGo
  (params (Motion%20Controller :type Scene%20Component%20Object%20Reference))
  ;[0.4121 0.7086 1] Let Go
  ;;[1 1 1] Determine which Hand to Let go
  (if (Utilities|IsValid (Variables|Default|GetSecondMotionController))
    (if (== (Variables|Default|GetSecondMotionController) Motion%20Controller)
      ;;[1 1 1] Two Hands: Second MC is Current -> Reset Second MC / Set Pivot to First
      (Variables|Default|SetSecondMotionController 0)
      (Variables|Default|SetPivot (Transformation|GetWorldLocation (Variables|Default|GetFirstMotionController)))
      (else
        ;;[1 1 1] Two Hands: First MC is Current -> Set Second to First / Set Pivot to new First
        (Variables|Default|SetFirstMotionController (Variables|Default|GetSecondMotionController))
        (Variables|Default|SetSecondMotionController 0)
        (Variables|Default|SetPivot (Transformation|GetWorldLocation (Variables|Default|GetFirstMotionController)))))
    ;;[1 1 1] Get MC Pawn / Decrement Climbing Hands
    (Math|Integer|DecrementInt (Variables|/Game/VirtualReality/VirtualRealityBP/Blueprints/MotionControllerPawn.MotionControllerPawn_C|GetClimbingHands (Variables|Default|GetMCPawn)) :!label _label)
    (elif (== Motion%20Controller (Variables|Default|GetFirstMotionController))
      ;;[1 1 1] One Hand: Reset All
      (Variables|Default|SetFirstMotionController 0)
      (Variables|Default|SetSecondMotionController 0)
      (Variables|Default|SetPivot "0, 0, 0")
      (goto _label))))

(fn ConstructionScript)