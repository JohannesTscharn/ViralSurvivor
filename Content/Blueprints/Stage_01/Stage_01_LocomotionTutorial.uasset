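; Stage 01 locomotion tutorial that teaches climbing, then a task with a bacterium and a wall light.
; Tick waits for the pawn to climb, then removes the first hint, plays a sound and lights a spotlight.
; A PopUp timeline scales in both objectives and, on its updates, manages the second hint and checks the wall light's buff counter to mark completion.
; A FogDensity timeline, played at BeginPlay and on completion, drives fog density.
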(event EventBeginPlay
  (Transformation|SetActorScale3D (Variables|Default|GetTutorialWallLight) "0, 0, 0")
  ;[1 1 1] Fog Density
  (Components|Timeline|PlayfromStart (Variables|Default|GetFogDensity))
  (Class|ExponentialHeightFogComponent|SetFogDensity (Variables|/Script/Engine.ExponentialHeightFog|GetComponent (Variables|Default|GetFog)) 0.0))

(event Collision|EventActorBeginOverlap
  (params (OtherActor :type Actor%20Object%20Reference)))

(event EventTick
  (params (DeltaSeconds :type Float%20%28single-precision%29))
  (bind _tutorialhandstext2 (Variables|Default|GetTutorialHandsText2))
  (bind _tutorialhandstext2_2 (Variables|Default|GetTutorialHandsText2))
  ;[1 1 1] Check if Pawn has Climbed
  (if (Variables|/Game/VirtualReality/VirtualRealityBP/Blueprints/MotionControllerPawn.MotionControllerPawn_C|GetHasClimbed (Variables|Default|GetMCPawn))
    ;[1 1 1] Disable Tutorial Hands + Text
    (if (Utilities|IsValid (Variables|Default|GetTutorialHandsText))
      (Actor|DestroyActor (Variables|Default|GetTutorialHandsText))
      (Transformation|SetRelativeScale3D (Variables|Default|GetCylinder) "0, 0, 0")
      ;[1 1 1] Sound
      (Audio|PlaySoundatLocation "/Game/Sound/TutorialSound.TutorialSound" (Transformation|GetActorLocation) "0, 0, 0" 1.0 1.0 0.0 0 0 0)
      ;[0.2764 0.6351 1] Enable Second Tutorial Step
      ;;[1 1 1] Enable Vein-Light
      (Rendering|Components|Light|SetIntensity (Variables|/Script/Engine.SpotLight|GetSpotLightComponent (Variables|Default|GetTutorialSpotlight)) 2.0)
      ;;[1 1 1] Pop Up next Objectives
      (bind _scale (Timeline|PopUp Play)
        (:Update
          (Transformation|SetActorScale3D (Variables|Default|GetTutorialWallLight) (Math|Conversions|ToVector(Float) _scale))
          (Transformation|SetActorScale3D (Variables|Default|GetTutorialBacterium) (* (Math|Conversions|ToVector(Float) _scale) 0.1))
          ;;[1 1 1] Check if bacterium has been picked up
          (if (Variables|/Game/Blueprints/Stage_01/PickupItem_BP.PickupItem_BP_C|GetPickedUp (Variables|Default|GetTutorialBacterium))
            ;;[1 1 1] Set Tutorial Text State
            (Transformation|SetActorScale3D _tutorialhandstext2_2 "0, 0, 0" :!label _label)
            (else
              (Utilities|IsValid (Variables|Default|GetTutorialBacterium)
                (:Is%20Valid
                  (goto _label))
                (:Is%20Not%20Valid
                  (Actor|DestroyActor _tutorialhandstext2_2)))))
          ;;[1 1 1] Check if Task Completed
          (if (> (Variables|/Game/Blueprints/Stage_01/BacteriumWallLight.BacteriumWallLight_C|GetBuffCounter (Variables|Default|GetTutorialWallLight)) 0.0)
            (Variables|Default|SetTutorialCompleted true)
            ;;[1 1 1] Destroy Text
            (Utilities|IsValid _tutorialhandstext2
              (:Is%20Valid
                (Actor|DestroyActor _tutorialhandstext2)
                ;;[1 1 1] Fog Density
                (bind _fogdensity (Timeline|FogDensity Play)
                  (:Update
                    (if (not (Variables|Default|GetTutorialSequence))
                      (Class|ExponentialHeightFogComponent|SetFogDensity (Variables|/Script/Engine.ExponentialHeightFog|GetComponent (Variables|Default|GetFog)) _fogdensity)))
                  (:Finished
                    (Variables|Default|SetTutorialSequence true))))
              (:Is%20Not%20Valid
                (Timeline|FogDensity Play)))))))))

(fn ConstructionScript)