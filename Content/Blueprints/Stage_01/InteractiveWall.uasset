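; Interactive wall actor for Stage 01 that glows when infected.
; It applies a configurable static mesh, then at BeginPlay creates a dynamic instance of Walls_Infected with its illumination zeroed.
; InfectWall sets the Infected flag and restarts the InfectionBuildUp timeline.
; Tick keeps that timeline playing, and its updates drive SecondaryIllum from the curve scaled by BaseIllumIntensity only while infected.
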(event EventBeginPlay
  (bind _wallmesh (Variables|Default|GetWallMesh))
  (Components|StaticMesh|SetStaticMesh (Variables|Default|GetWallMesh) (Variables|Default|GetStaticMesh))
  (bind _returnvalue (Rendering|Material|CreateDynamicMaterialInstance _wallmesh 0 "/Game/Assets/Materials/Stage_01/Walls_Infected.Walls_Infected" "None" :!class /Script/Engine.PrimitiveComponent))
  (bind _output_get (Variables|Default|SetMaterialInstance _returnvalue))
  (Rendering|Material|SetMaterial _wallmesh 1 _output_get)
  (Rendering|Material|SetScalarParameterValue (Variables|Default|GetMaterialInstance) "SecondaryIllum" 0.0 :!class /Script/Engine.MaterialInstanceDynamic))

(event Collision|EventActorBeginOverlap
  (params (OtherActor :type Actor%20Object%20Reference)))

(event EventTick
  (params (DeltaSeconds :type Float%20%28single-precision%29))
  (bind _illum (Timeline|InfectionBuildUp Play)
    (:Update
      (if (Variables|Default|GetInfected)
        (Rendering|Material|SetScalarParameterValue (Variables|Default|GetMaterialInstance) "SecondaryIllum" (* (Variables|Default|GetBaseIllumIntensity) _illum) :!class /Script/Engine.MaterialInstanceDynamic)))))

(fn ConstructionScript
  (Components|StaticMesh|SetStaticMesh (Variables|Default|GetWallMesh) (Variables|Default|GetStaticMesh)))

(fn InfectWall
  (Components|Timeline|PlayfromStart (Variables|Default|GetInfectionBuildUp))
  (Variables|Default|SetInfected true))