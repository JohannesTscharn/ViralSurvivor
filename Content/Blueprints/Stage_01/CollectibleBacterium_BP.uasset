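; Collectible bacterium actor for Stage 01 that the player picks up by touching it with either VR motion controller.
; It copies the left and right controller references from the Stage 01 controller Blueprint on BeginPlay and refreshes them every Tick.
; An overlap with either controller increments the stage controller's collected-bacteria counter, then destroys the bacterium.
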(event EventBeginPlay
  (bind _stage_01_controller_bp (Variables|Default|GetStage_01_Controller_BP))
  ;[1 1 1] Get Both Controller References from Stage_01_Controller
  (Variables|Default|SetMotionController_R (Variables|/Game/Blueprints/Stage_01/Stage_01_Controller_BP.Stage_01_Controller_BP_C|GetBP_MotionController_R _stage_01_controller_bp))
  (Variables|Default|SetMotionController_L (Variables|/Game/Blueprints/Stage_01/Stage_01_Controller_BP.Stage_01_Controller_BP_C|GetBP_MotionController_L _stage_01_controller_bp)))

(event Collision|EventActorBeginOverlap
  (params (OtherActor :type Actor%20Object%20Reference))
  ;[1 1 1] If Other is HMD Pawn Check
  (if (== OtherActor (Variables|Default|GetMotionController_R))
    ;[1 1 1] Increment Counter
    (Default|IncrementBactCollected (Variables|Default|GetStage_01_Controller_BP) :!label _label)
    ;[1 1 1] Destroy (Self)
    (Actor|DestroyActor)
    (elif (== OtherActor (Variables|Default|GetMotionController_L))
      (goto _label))))

(event EventTick
  (params (DeltaSeconds :type Float%20%28single-precision%29))
  (bind _stage_01_controller_bp (Variables|Default|GetStage_01_Controller_BP))
  ;[1 1 1] Get Both Controller References from Stage_01_Controller
  (Variables|Default|SetMotionController_R (Variables|/Game/Blueprints/Stage_01/Stage_01_Controller_BP.Stage_01_Controller_BP_C|GetBP_MotionController_R _stage_01_controller_bp))
  (Variables|Default|SetMotionController_L (Variables|/Game/Blueprints/Stage_01/Stage_01_Controller_BP.Stage_01_Controller_BP_C|GetBP_MotionController_L _stage_01_controller_bp)))

(fn ConstructionScript)