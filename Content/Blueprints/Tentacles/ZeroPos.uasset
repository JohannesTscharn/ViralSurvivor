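; ZeroPos is an actor in the Tentacles folder that drifts randomly around its starting point.
; BeginPlay stores the start location and picks a target offset in Y and Z within RndMoveRange, keeping X fixed.
; Tick eases toward it with VInterpTo at a speed re-randomized every frame, picking a new target once within tolerance.
; It reads world location but writes relative location, which differ if attached.
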(event EventBeginPlay
  (bind _rndmove_range (Variables|Default|GetRndMove_Range))
  (Variables|Default|SetStartPos (Transformation|GetActorLocation self))
  (Variables|Default|SetRandomPos (Math|Vector|MakeVector (.X (Math|Vector|BreakVector (Variables|Default|GetStartPos))) (Math|Random|RandomFloatinRange (- (.Y (Math|Vector|BreakVector (Variables|Default|GetStartPos))) _rndmove_range) (+ (.Y (Math|Vector|BreakVector (Variables|Default|GetStartPos))) _rndmove_range)) (Math|Random|RandomFloatinRange (- (.Z (Math|Vector|BreakVector (Variables|Default|GetStartPos))) _rndmove_range) (+ (.Z (Math|Vector|BreakVector (Variables|Default|GetStartPos))) _rndmove_range)))))

(event EventTick
  (params (DeltaSeconds :type Float%20%28single-precision%29))
  (bind _startpos (Variables|Default|GetStartPos))
  (bind _rndmove_range (Variables|Default|GetRndMove_Range))
  (bind (_x _y _z) (Math|Vector|BreakVector _startpos))
  (Transformation|SetActorRelativeLocation (Math|Interpolation|VInterpTo (Transformation|GetActorLocation) (Variables|Default|GetRandomPos) (Utilities|Time|GetWorldDeltaSeconds) (Math|Random|RandomFloatinRange 0.1 0.35)))
  (if (Math|Vector|Equal(Vector) (Transformation|GetActorLocation) (Variables|Default|GetRandomPos) 5.0)
    (Variables|Default|SetRandomPos (Math|Vector|MakeVector _x (Math|Random|RandomFloatinRange (- _y _rndmove_range) (+ _y _rndmove_range)) (Math|Random|RandomFloatinRange (- _z _rndmove_range) (+ _z _rndmove_range))))))

(fn ConstructionScript)