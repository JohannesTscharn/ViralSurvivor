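; LineTracer is a component that supplies a ray hit point to its owning BP_MotionController.
; Each tick it runs a debug-drawn Visibility trace from the owner's location, skipping IgnoreActors, and writes the hit location to RayHit.
; The trace end is the forward vector times a fixed length without the start location added, so it is relative to world origin.
; NewFunction_0 is a stub containing only a cast.
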(event EventBeginPlay)

(event EventTick
  (params (DeltaSeconds :type Float%20%28single-precision%29))
  (bind _returnvalue (Components|GetOwner))
  (bind _outhit (Collision|LineTraceByChannel (Transformation|GetActorLocation _returnvalue) (* (Transformation|GetActorForwardVector _returnvalue) 1e+03) "TraceTypeQuery1" false (Variables|Default|GetIgnoreActors) "ForOneFrame"))
  (bind _asbp_motion_controller (Utilities|Casting|CastToBP_MotionController (Components|GetOwner)))
  (Variables|/Game/VirtualReality/VirtualRealityBP/Blueprints/BP_MotionController.BP_MotionController_C|SetRayHit _asbp_motion_controller (.Location (Collision|BreakHitResult _outhit))))

(fn NewFunction0
  (params (Object :type Object%20Object%20Reference))
  (Utilities|Casting|CastToBP_MotionController Object))