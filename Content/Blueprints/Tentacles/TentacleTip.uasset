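; TentacleTip is the actor at a tentacle's tip, which eases toward a target point each frame.
; On Tick it measures its distance to the PlayerPos actor, then runs FollowTarget.
; While RayHit is non-zero and that distance is under MaxDist, it interpolates toward RayHit with VInterpTo.
; Otherwise it drifts back to the ZeroPos actor's location at the same slow speed.
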(event EventTick
  (params (DeltaSeconds :type Float%20%28single-precision%29))
  (Variables|Default|SetPlayerDist (Math|Vector|Distance(Vector) (Transformation|GetActorLocation) (Transformation|GetActorLocation (Variables|Default|GetPlayerPos))))
  (CallFunction|FollowTarget))

(fn ConstructionScript)

(fn FollowTarget
  (if (Math|Vector|Equal(Vector) (Variables|Default|GetRayHit) "0, 0, 0" 0.0001)
    (Transformation|SetActorLocation (Math|Interpolation|VInterpTo (Transformation|GetActorLocation) (Transformation|GetActorLocation (Variables|Default|GetZeroPos)) (Utilities|Time|GetWorldDeltaSeconds) 0.5) false false :!label _label)
    (elif (< (Variables|Default|GetPlayerDist) (Variables|Default|GetMaxDist))
      (Transformation|SetActorLocation (Math|Interpolation|VInterpTo (Transformation|GetActorLocation) (Variables|Default|GetRayHit) (Utilities|Time|GetWorldDeltaSeconds) 0.5) false false)
      (else
        (goto _label)))))