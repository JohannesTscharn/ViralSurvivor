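; Climbable VR vein actor whose construction script builds fixed-length, collidable spline mesh sections along a spline.
; Unwired EventGraph logic would animate vein material glow on activation, then light a wall or child wall light.
; Also unwired, grab logic tracks two motion controllers and offsets the pawn against the latest grip's pivot.
; Tick, Climb and LetGo are empty, so only the spline building runs.
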(event EventBeginPlay)

(event Collision|EventActorBeginOverlap
  (params (OtherActor :type Actor%20Object%20Reference)))

(event EventTick
  (params (DeltaSeconds :type Float%20%28single-precision%29)))

(event EventClimb
  (params (Motion%20Controller :type Scene%20Component%20Object%20Reference)))

(event EventLetGo
  (params (Motion%20Controller :type Scene%20Component%20Object%20Reference)))

(fn ConstructionScript
  (bind _spline (Variables|Default|GetSpline))
  (bind _spline_2 (Variables|Default|GetSpline))
  ;[0.4688 0.7795 1] Loop over all Spline points
  (for _index (range 0 (Math|Float|Truncate (/ (Spline|GetSplineLength (Variables|Default|GetSpline)) (Variables|Default|GetSectionLength))))
    ;;[1 1 1] Add and configure SplineMesh Component
    (bind _returnvalue (AddComponent|AddSplineMeshComponent false))
    (Utilities|Array|Add (Variables|Default|GetSplineMeshes) _returnvalue)
    (SplineMesh|SetForwardAxis _returnvalue "Z" true)
    (Collision|SetCollisionEnabled _returnvalue "QueryAndPhysics")
    (SplineMesh|SetStartandEnd _returnvalue (Spline|GetLocationatDistanceAlongSpline _spline_2 (* _index (Variables|Default|GetSectionLength)) "Local") (Math|Vector|ClampVectorSize (Spline|GetTangentatDistanceAlongSpline _spline_2 (* _index (Variables|Default|GetSectionLength)) "Local") 0.0 (Variables|Default|GetSectionLength)) (Spline|GetLocationatDistanceAlongSpline _spline (* (+ _index 1) (Variables|Default|GetSectionLength)) "Local") (Math|Vector|ClampVectorSize (Spline|GetTangentatDistanceAlongSpline _spline (* (+ _index 1) (Variables|Default|GetSectionLength)) "Local") 0.0 (Variables|Default|GetSectionLength)) true :!class /Script/Engine.SplineMeshComponent)))